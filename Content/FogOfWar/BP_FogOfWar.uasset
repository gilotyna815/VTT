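; Fog-of-war actor that masks the view with post-process materials based on what each BP_VTTPawn sees.
; InitializeFog, given 2, stacks field-of-view (fed by pawn cube render targets) and feedback materials per pawn, plus one fog material bounded by FogVolume.
; Tick updates observer locations at material slot 3^index, which matches the stacking only for two pawns.
; The Observers list is unread, and shadow-mask render-target code is disconnected.
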(event `InitializeFog`
  (params (Number :type Integer))
  (bind (_returnvalue_x _returnvalue_y _returnvalue_z) (`KismetMathLibrary.BreakVector` (`SceneComponent.K2_GetComponentLocation` (`self.FogVolume`))))
  (bind _weightedblendables_array (break `WeightedBlendables` (break `PostProcessSettings` (`PostProcessComponent.Settings` (`self.PostProcess`)))))
  (bind _weightedblendables_array_2 (break `WeightedBlendables` (break `PostProcessSettings` (`PostProcessComponent.Settings` (`self.PostProcess`)))))
  (bind _weightedblendables_array_3 (break `WeightedBlendables` (break `PostProcessSettings` (`PostProcessComponent.Settings` (`self.PostProcess`)))))
  (bind (_returnvalue_x_2 _returnvalue_y_2 _returnvalue_z_2) (`KismetMathLibrary.BreakVector` (* (`BoxComponent.GetScaledBoxExtent` (`self.FogVolume`)) 2)))
  ;[1 0 0] Begin Play
  (if (== Number 2)
    (`/Engine/EditorBlueprintResources/StandardMacros.DoOnce` false
      (:`Completed`
        (`|ExecutionSequence`
          (:`then_0`
            ;;[0 1 1] Managing Observers list
            (bind _outactors (`GameplayStatics.GetAllActorsOfClass` "/Game/FogOfWar/BP_VTTPawn.BP_VTTPawn_C"))
            (bind _output_get (set `self.Pawns` _outactors))
            (for _array_element _output_get
              (bind _returnvalue (`KismetMaterialLibrary.CreateDynamicMaterialInstance` "/Game/FogOfWar/PPM_FieldOfView.PPM_FieldOfView"))
              (`MaterialInstanceDynamic.SetTextureParameterValue` _returnvalue "RenderTargetCube" (`/Game/FogOfWar/BP_VTTPawn.RenderTargetCube` _array_element))
              (`MaterialInstanceDynamic.SetTextureParameterValue` _returnvalue "RenderTargetCube1" (`/Game/FogOfWar/BP_VTTPawn.RenderTargetCube_0` _array_element))
              (`KismetArrayLibrary.Array_Add` _weightedblendables_array_3 (make `WeightedBlendable` 1.0 _returnvalue))
              (bind (_returnvalue_x_3 _returnvalue_y_3 _returnvalue_z_3) (`KismetMathLibrary.BreakVector` (`SceneComponent.K2_GetComponentLocation` (`/Game/FogOfWar/BP_VTTPawn.SceneCaptureComponentCube` _array_element))))
              (`MaterialInstanceDynamic.SetVectorParameterValue` _returnvalue "ObserversLocation" (make `LinearColor` _returnvalue_x_3 _returnvalue_y_3 _returnvalue_z_3 1.0))
              (bind _returnvalue_2 (`KismetMaterialLibrary.CreateDynamicMaterialInstance` "/Game/FogOfWar/PPM_Feedback.PPM_Feedback"))
              (`KismetArrayLibrary.Array_Add` _weightedblendables_array_2 (make `WeightedBlendable` 1.0 _returnvalue_2))))
          (:`then_1`
            ;;[0 1 0] Create PostProcessMaterial
            (bind _returnvalue_3 (`KismetMaterialLibrary.CreateDynamicMaterialInstance` "/Game/FogOfWar/PPM_FogOfWar.PPM_FogOfWar"))
            (bind _output_get_2 (set `self.PostProcessMaterialInstance` _returnvalue_3))
            (`KismetArrayLibrary.Array_Add` _weightedblendables_array (make `WeightedBlendable` 1.0 _output_get_2))
            (`MaterialInstanceDynamic.SetVectorParameterValue` _output_get_2 "FogColor" (`self.FogColor`))
            (`MaterialInstanceDynamic.SetDoubleVectorParameterValue` _output_get_2 "FogOrigin" (`KismetMathLibrary.MakeVector4` _returnvalue_x _returnvalue_y _returnvalue_z))
            (`MaterialInstanceDynamic.SetDoubleVectorParameterValue` _output_get_2 "FogBounds" (`KismetMathLibrary.MakeVector4` _returnvalue_x_2 _returnvalue_y_2 _returnvalue_z_2))
            (`MaterialInstanceDynamic.SetScalarParameterValue` _output_get_2 "FogOpacity" (`KismetMathLibrary.SelectFloat` 0.825 1.0))))))))

(event `self.ReceiveBeginPlay`
  ;[1 0 0] Begin Play
  (`parent.ReceiveBeginPlay`))

(event `AddObserver`
  (params (Observer :type "/Game/VTTObject/BP_VTTObject Object Reference"))
  ;[1 0 0] Begin Play
  ;;[0 1 1] Managing Observers list
  (`KismetArrayLibrary.Array_AddUnique` (`self.Observers`) Observer))

(event `RemoveObserver`
  (params (Observer :type "/Game/VTTObject/BP_VTTObject Object Reference"))
  ;[1 0 0] Begin Play
  ;;[0 1 1] Managing Observers list
  (`KismetArrayLibrary.Array_RemoveItem` (`self.Observers`) Observer))

(event `self.ReceiveTick`
  (params (DeltaSeconds :type "Float (single-precision)"))
  (bind _weightedblendables_array (break `WeightedBlendables` (break `PostProcessSettings` (`PostProcessComponent.Settings` (`self.PostProcess`)))))
  (for (_array_element _array_index) (`self.Pawns`)
    (bind (_output_weight _output_object) (break `WeightedBlendable` (`|GetArrayItem` _weightedblendables_array (`KismetMathLibrary.FTrunc` (`KismetMathLibrary.MultiplyMultiply_FloatFloat` 3.0 (`KismetMathLibrary.Conv_IntToDouble` _array_index))))))
    ;[1 0 0] Begin Play
    (bind _asmaterial_instance_dynamic (cast `MaterialInstanceDynamic` _output_object))
    (bind (_returnvalue_x _returnvalue_y _returnvalue_z) (`KismetMathLibrary.BreakVector` (`SceneComponent.K2_GetComponentLocation` (`/Game/FogOfWar/BP_VTTPawn.SceneCaptureComponentCube` _array_element))))
    (`MaterialInstanceDynamic.SetVectorParameterValue` _asmaterial_instance_dynamic "ObserversLocation" (make `LinearColor` _returnvalue_x _returnvalue_y _returnvalue_z 1.0))))

(fn `CreateRenderTargetCube`
  (params (Size :type Integer))
  (returns (RenderTargetCube :type "TextureRenderTargetCube Object Reference"))
  (bind _returnvalue (`KismetSystemLibrary.GetClassDisplayName` (`GameplayStatics.GetObjectClass` self)))
  (bind _returnvalue_2 (`AssetToolsHelpers.GetAssetTools`))
  (bind _returnvalue_3 (`AssetTools.DuplicateAsset` _returnvalue_2 "RenderTargetCube" (`KismetStringLibrary.Concat_StrStr` (`KismetStringLibrary.Left` _returnvalue (`KismetStringLibrary.FindSubstring` _returnvalue "/" false true)) "/Captures") null))
  (bind _astexture_render_target_cube (cast `TextureRenderTargetCube` _returnvalue_3))
  (set `TextureRenderTargetCube.SizeX` Size _astexture_render_target_cube)
  (return _astexture_render_target_cube))

(fn `UserConstructionScript`
  (`parent.UserConstructionScript`)
  (`SceneComponent.SetWorldScale3D` (`self.StaticMesh`) (1.0 1.0 1.0)))