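; Test observer actor for the fog of war system that registers itself with every BP_FogOfWar on BeginPlay or BecomeObserver.
; UpdateLineOfSight sweeps line traces over a sphere by inclination and azimuth, stores distance and angles in Hits, then fires OnLineOfSightUpdated, guarded by a Busy flag.
; The post-process material and render target setup, and this graph's calls to UpdateLineOfSight, are disconnected.
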(event `self.ReceiveBeginPlay`
  (`|ExecutionSequence`
    (:`then_0`
      (`parent.ReceiveBeginPlay`))
    (:`then_2`
      (bind _outactors (`GameplayStatics.GetAllActorsOfClass` "/Game/FogOfWar/BP_FogOfWar.BP_FogOfWar_C" :!label _label))
      (for _array_element _outactors
        (`/Game/FogOfWar/BP_FogOfWar.AddObserver` _array_element self)))))

(event `BecomeObserver`
  (goto _label))

(event `self.ReceiveTick`
  (params (DeltaSeconds :type "Float (single-precision)")))

(fn `UpdateLineOfSight`
  (locals (SightVector :type "Vector Structure") (Inclination :type "Float (double-precision)") (Azimuth :type "Float (double-precision)"))
  (bind _returnvalue (`self.K2_GetActorLocation`))
  (if (not (`self.Busy`))
    (set `self.Busy` true)
    (`KismetArrayLibrary.Array_Clear` (`self.Hits`))
    (set `local.Inclination` 0.0)
    (while (<= (`local.Inclination`) 180.0)
      (set `local.Azimuth` 0.0)
      (while (<= (`local.Azimuth`) (`KismetMathLibrary.SelectFloat` 0.0 360.0 (or (== (`local.Inclination`) 0.0) (== (`local.Inclination`) 180.0))))
        (set `local.SightVector` (`KismetMathLibrary.GreaterGreater_VectorRotator` (`SceneComponent.GetUpVector` (`self.Scene`)) (`KismetMathLibrary.MakeRotator` 0.0 (* (`local.Inclination`) -1.0) (`local.Azimuth`))))
        (bind _outhit (`KismetSystemLibrary.LineTraceSingle` :`Start` _returnvalue :`End` (+ _returnvalue (* (`local.SightVector`) (`self.RangeOfSight`))) :`TraceChannel` "TraceTypeQuery1" :`bTraceComplex` true :`DrawDebugType` "ForOneFrame"))
        (`KismetArrayLibrary.Array_Add` (`self.Hits`) (make `/Game/FogOfWar/S_LineOfSightPoint` (`KismetMathLibrary.SelectFloat` (`.Distance` (`GameplayStatics.BreakHitResult` _outhit)) (`self.RangeOfSight`) (`GameplayStatics.BreakHitResult` _outhit)) (`local.Inclination`) (`local.Azimuth`)))
        (set `local.Azimuth` (+ (`local.Azimuth`) (`self.LineOfSightPrecision`))))
      (set `local.Inclination` (+ (`local.Inclination`) (`self.LineOfSightPrecision`))))
    (`self.OnLineOfSightUpdated`)
    (set `self.Busy` false)))

(fn `UserConstructionScript`
  (`parent.UserConstructionScript`))