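; Virtual tabletop pawn that captures its surroundings into two cube render targets, apparently for field-of-view fog of war.
; BeginPlay binds both captures, initializes every BP_FogOfWar if this is the only pawn, and hides POV and gizmo actors from the first capture.
; CreateCubeRenderTarget loads or duplicates a per-pawn cube target asset through asset tools.
; Its only call, like the post-process shadow-mask setup, sits in disconnected nodes.
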(event `self.ReceiveTick`
  (params (DeltaSeconds :type "Float (single-precision)")))

(event `self.ReceiveBeginPlay`
  (`|ExecutionSequence`
    (:`then_0`
      (set `SceneCaptureComponentCube.TextureTarget` (`self.RenderTargetCube`) (`self.SceneCaptureComponentCube`))
      (set `SceneCaptureComponentCube.TextureTarget` (`self.RenderTargetCube_0`) (`self.SceneCaptureComponentCube1`)))
    (:`then_1`
      (bind _outactors (`GameplayStatics.GetAllActorsOfClass` "BP_VTTPawn_C"))
      (bind _returnvalue (`KismetArrayLibrary.Array_Length` _outactors))
      (if (== _returnvalue 1)
        (bind _outactors_2 (`GameplayStatics.GetAllActorsOfClass` "/Game/FogOfWar/BP_FogOfWar.BP_FogOfWar_C"))
        (for _array_element _outactors_2
          (`/Game/FogOfWar/BP_FogOfWar.InitializeFog` _array_element _returnvalue))))
    (:`then_2`
      (bind _outactors_3 (`GameplayStatics.GetAllActorsOfClass` "/Game/GameMode/BP_VTTPOV.BP_VTTPOV_C"))
      (bind _output_get (set `self.DoNotCaptureActors` _outactors_3))
      (bind _outactors_4 (`GameplayStatics.GetAllActorsOfClass` "/Game/Gizmo/BP_Gizmo.BP_Gizmo_C"))
      (`KismetArrayLibrary.Array_Append` _output_get _outactors_4)
      (set `SceneCaptureComponent.HiddenActors` (`self.DoNotCaptureActors`) (`self.SceneCaptureComponentCube`)))))

(fn `CreateCubeRenderTarget`
  (returns (NewRenderTargetCube :type "TextureRenderTargetCube Object Reference"))
  (bind _rendertargetcube (`self.RenderTargetCube`))
  (bind _returnvalue (`KismetStringLibrary.Concat_StrStr` "CRT_FieldOfView_" (`KismetSystemLibrary.GetObjectName` self)))
  (bind _returnvalue_2 (`AssetToolsHelpers.GetAssetTools`))
  (bind _returnvalue_3 (`AssetRegistry.GetAssetByObjectPath` (`AssetRegistryHelpers.GetAssetRegistry`) (`KismetSystemLibrary.MakeLiteralName` (`KismetStringLibrary.Conv_StringToName` (`KismetStringLibrary.Concat_StrStr` "/Game/Captures" "/" _returnvalue))) false))
  (if (`AssetRegistryHelpers.IsValid` _returnvalue_3)
    (bind _astexture_render_target_cube (cast `TextureRenderTargetCube` (`AssetRegistryHelpers.GetAsset` _returnvalue_3))
      (:`then`
        (set `self.RenderTargetCube` _astexture_render_target_cube))
      (:`CastFailed`
        (bind _returnvalue_4 (`AssetTools.DuplicateAsset` _returnvalue_2 _returnvalue "/Game/Captures" "/Game/FogOfWar/CRT_FieldOfView.CRT_FieldOfView" :!label _label))
        (bind _astexture_render_target_cube_2 (cast `TextureRenderTargetCube` _returnvalue_4))
        (set `self.RenderTargetCube` _astexture_render_target_cube_2)))
    (else
      (goto _label)))
  (set `TextureRenderTargetCube.SizeX` 512 _rendertargetcube)
  (bind _output_get (set `SceneCaptureComponentCube.TextureTarget` _rendertargetcube (`self.SceneCaptureComponentCube`)))
  (return _output_get))

(fn `UserConstructionScript`
  (`parent.UserConstructionScript`))