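; Game instance for a VTT project that owns the persistent save data object.
; On Init or LoadSaveData, it loads a BP_VTTGameSave from a fixed test slot, or creates a new one if none exists.
; SaveSaveData calls UpdateSaveData, currently an empty event, then writes to the slot synchronously or asynchronously.
; Only a failed synchronous save prints an on-screen error.
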(event `self.ReceiveInit`
  (`parent.ReceiveInit`)
  ;[0.6706 0.8706 0.2353] Load Save Data
  (bind _returnvalue (`GameplayStatics.DoesSaveGameExist` (`self.TestGameSaveSlot`) :!label _label))
  (if _returnvalue
    (bind _returnvalue_2 (`GameplayStatics.LoadGameFromSlot` (`self.TestGameSaveSlot`)))
    (bind _asbp_vttgame_save (cast `/Game/SaveSystem/BP_VTTGameSave` _returnvalue_2))
    (set `self.SaveData` _asbp_vttgame_save)
    (else
      (bind _returnvalue_3 (`GameplayStatics.CreateSaveGameObject` "/Game/SaveSystem/BP_VTTGameSave.BP_VTTGameSave_C"))
      (set `self.SaveData` _returnvalue_3))))

(event `LoadSaveData`
  ;[0.6706 0.8706 0.2353] Load Save Data
  (goto _label))

(event `SaveSaveData`
  (params (Async :type Boolean))
  (bind _testgamesaveslot (`self.TestGameSaveSlot`))
  (bind _savedata (`self.SaveData`))
  ;[0.898 0.5765 0.2745] Save Save Data
  (`self.UpdateSaveData`)
  (if Async
    (`AsyncActionHandleSaveGame.AsyncSaveGameToSlot` _savedata _testgamesaveslot)
    (else
      (bind _returnvalue (`GameplayStatics.SaveGameToSlot` _savedata _testgamesaveslot))
      (if (not _returnvalue)
        (`KismetSystemLibrary.PrintString` "Couldn't save data to slot, engine error." true true (struct :`R` 1.0 :`A` 1.0) 20.0)))))

(event `UpdateSaveData`)