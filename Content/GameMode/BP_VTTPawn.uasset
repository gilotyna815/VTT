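; BP_VTTPawn is the player pawn for a virtual tabletop, acting as a camera whose view can be saved and restored.
; BeginPlay shows the mouse cursor and enables input.
; Save data pairs the actor's location and scale with the controller's control rotation; loading reapplies both transform and control rotation.
; A debug O key spawns a cone BP_VTTObject at the pawn, taking its SaveID from the map via BPI_SaveIDManager.
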(event `self.ReceiveBeginPlay`
  (bind _returnvalue (`GameplayStatics.GetPlayerController` 0))
  (set `PlayerController.bShowMouseCursor` true _returnvalue)
  (`self.EnableInput` _returnvalue))

(event `Key|O`
  (params (Key :type "Key Structure"))
  ;[1 1 1] Spawn test VTTObject
  (:`Pressed`
    (bind _outactors (`GameplayStatics.GetAllActorsWithInterface` "/Game/SaveSystem/BPI_SaveIDManager.BPI_SaveIDManager_C"))
    (bind _saveid (message `/Game/SaveSystem/BPI_SaveIDManager.AssignSaveID` (`|GetArrayItem` _outactors)))
    (bind _returnvalue (`|SpawnActorFromClass` "/Game/VTTObject/BP_VTTObject.BP_VTTObject_C" (`self.GetTransform`) "AlwaysSpawn" "MultiplyWithRoot" null _saveid null))
    (`StaticMeshComponent.SetStaticMesh` (`/Game/VTTObject/BP_VTTObject.StaticMesh` _returnvalue) "/Engine/BasicShapes/Cone.Cone")))

(fn `GetSaveData`
  (returns (SaveData :type "/Game/SaveSystem/S_CameraSave Structure"))
  (bind (_returnvalue_location _returnvalue_rotation _returnvalue_scale) (`KismetMathLibrary.BreakTransform` (`self.GetTransform`)))
  (return (make `/Game/SaveSystem/S_CameraSave` (`KismetMathLibrary.MakeTransform` _returnvalue_location (`Controller.GetControlRotation` (`self.GetController`)) _returnvalue_scale))))

(fn `LoadSaveData`
  (params (SaveData :type "/Game/SaveSystem/S_CameraSave Structure"))
  (`self.K2_SetActorTransform` SaveData_CameraTransform_3_887DF81D48F00F7B09F709AF7048273C false true)
  (`Controller.SetControlRotation` (`self.GetController`) (.rotation SaveData_CameraTransform_3_887DF81D48F00F7B09F709AF7048273C)))

(fn `UserConstructionScript`)