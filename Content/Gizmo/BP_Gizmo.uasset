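; Translation gizmo actor for selecting BP_VTTObjects with the mouse and dragging them along X, Y or Z.
; Clicked objects attach to the gizmo, with Shift for multi-select, and it jumps to the newest by briefly detaching the selection.
; Axis grabs open a Tick gate moving it via cursor line-plane intersection; mouse release updates object transforms.
; Tick also scales it by square root of distance to the VTT pawn to steady screen size.
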(event `self.ReceiveBeginPlay`
  (bind _returnvalue (`GameplayStatics.GetPlayerController` 0))
  ;[0.005605 0.4508 0.956] Begin Play
  (`|ExecutionSequence`
    (:`then_0`
      ;;[1 0 0] Enable input
      (set `PlayerController.bShowMouseCursor` true _returnvalue)
      (`self.EnableInput` _returnvalue))
    (:`then_1`
      ;;[0.3613 0.002428 0.6514] Caching player camera for scaling
      (bind _outactors (`GameplayStatics.GetAllActorsOfClass` "/Game/GameMode/BP_VTTPawn.BP_VTTPawn_C"))
      (set `self.Camera` (`|GetArrayItem` _outactors)))))

(event `Key|LeftShift`
  (params (Key :type "Key Structure"))
  ;[0 1 0] Try to attach selected object
  ;;[1 0 0] If shift is down, select multiple actors
  (:`Pressed`
    (set `self.IsLeftShiftDown` true))
  (:`Released`
    (set `self.IsLeftShiftDown` false)))

(event `Key|RightShift`
  (params (Key :type "Key Structure"))
  ;[0 1 0] Try to attach selected object
  ;;[1 0 0] If shift is down, select multiple actors
  (:`Pressed`
    (set `self.IsRightShiftDown` true))
  (:`Released`
    (set `self.IsRightShiftDown` false)))

(event `Key|LeftMouseButton`
  (params (Key :type "Key Structure"))
  (bind (_bblockinghit _binitialoverlap _time _distance _location _impactpoint _normal _impactnormal _physmat _hitactor) (`GameplayStatics.BreakHitResult` (`PlayerController.GetHitResultUnderCursorForObjects` (`GameplayStatics.GetPlayerController` 0) (`|MakeArray` "ObjectTypeQuery8" :!type "EObjectTypeQuery Enum") true)))
  ;[0 1 0] Try to attach selected object
  (:`Pressed`
    (if (and _bblockinghit (`KismetSystemLibrary.IsValid` _hitactor))
      (bind _asbp_vttobject (cast `/Game/VTTObject/BP_VTTObject` _hitactor))
      (if (`/Game/VTTObject/BP_VTTObject.Selectable` _asbp_vttobject)
        ;;[1 0 0] If shift is down, select multiple actors
        (if (not (or (`self.IsLeftShiftDown`) (`self.IsRightShiftDown`)))
          (`self.DetachAllSelectedObjects`))
        (`self.TryToAddToSelection` _asbp_vttobject)))))

(event `Key|LeftMouseButton`
  (params (Key :type "Key Structure"))
  (bind (_returnvalue_x _returnvalue_y _returnvalue_z) (`KismetMathLibrary.BreakVector` (`self.K2_GetActorLocation` self)))
  (bind (_worldlocation _worlddirection) (`PlayerController.DeprojectMousePositionToWorld` (`GameplayStatics.GetPlayerController` 0)))
  (bind (_bblockinghit _binitialoverlap _time _distance _location _impactpoint _normal _impactnormal _physmat _hitactor _hitcomponent) (`GameplayStatics.BreakHitResult` (`PlayerController.GetHitResultUnderCursorForObjects` (`GameplayStatics.GetPlayerController` 0) (`|MakeArray` "ObjectTypeQuery7" :!type "EObjectTypeQuery Enum") true)))
  (bind (_t _intersection) (`KismetMathLibrary.LinePlaneIntersection_OriginNormal` (`PlayerCameraManager.GetCameraLocation` (`GameplayStatics.GetPlayerCameraManager` 0)) (+ _worldlocation (* _worlddirection (`self.DistanceOfGrab`))) (`self.K2_GetActorLocation`) (`self.PlaneNormal`)))
  ;[1 0 0] When Player clicks on this gizmo
  (:`Pressed`
    (if _bblockinghit
      (switch `EAxis` (`self.GetGrabbedAxis` _hitcomponent)
        (:`X`
          _)
        (:`Y`
          _)
        (:`Z`
          _))
      (set `self.AxisDragged` _hitcomponent)
      (goto _label :!via `Open`)))
  (:`Released`
    ;;[0 0 0] Reset
    (set `self.AxisDragged` null)
    (`self.Update Transforms Of Selected Objects`)
    (goto _label :!via `Close`)))

(event `self.ReceiveTick`
  (params (DeltaSeconds :type "Float (single-precision)"))
  (bind (_returnvalue_x _returnvalue_y _returnvalue_z) (`KismetMathLibrary.BreakVector` (`self.K2_GetActorLocation` self)))
  (bind (_worldlocation _worlddirection) (`PlayerController.DeprojectMousePositionToWorld` (`GameplayStatics.GetPlayerController` 0)))
  (bind _returnvalue (* (`KismetMathLibrary.Sqrt` (`self.GetDistanceTo` (`self.Camera`))) (`self.GizmoScale`)))
  (bind (_t _intersection) (`KismetMathLibrary.LinePlaneIntersection_OriginNormal` (`PlayerCameraManager.GetCameraLocation` (`GameplayStatics.GetPlayerCameraManager` 0)) (+ _worldlocation (* _worlddirection (`self.DistanceOfGrab`))) (`self.K2_GetActorLocation`) (`self.PlaneNormal`)))
  ;[0.000304 0.5457 0.2747] Tick
  (`|ExecutionSequence`
    (:`then_0`
      ;;[0 0.3845 1] Move Gizmo
      (`/Engine/EditorBlueprintResources/StandardMacros.Gate` true :!label _label
        (:`Exit`
          (switch `EAxis` (`self.GetGrabbedAxis` (`self.AxisDragged`))
            (:`None`
              (goto _label :!via `Close`))
            (:`X`
              ;;;[1 0.9867 0] Plane Normal
              (set `self.PlaneNormal` (0.0 1.0 1.0))
              ;;;[1 0.9097 0] New Location
              (set `self.NewLocation` (`KismetMathLibrary.MakeVector` (.x _intersection) _returnvalue_y _returnvalue_z)))
            (:`Y`
              (set `self.PlaneNormal` (1.0 0.0 1.0))
              (set `self.NewLocation` (`KismetMathLibrary.MakeVector` _returnvalue_x (.y _intersection) _returnvalue_z)))
            (:`Z`
              (set `self.PlaneNormal` (1.0 1.0 0.0))
              (set `self.NewLocation` (`KismetMathLibrary.MakeVector` _returnvalue_x _returnvalue_y (.z _intersection)))))
          (`self.K2_SetActorLocation` (`self.NewLocation`) false true))))
    (:`then_1`
      ;;[0.6867 0.016 0.1329] Rescale gizmo depending on distance to camera to preserve same size on screen
      (`SceneComponent.SetWorldScale3D` (`self.GizmoRoot`) (`KismetMathLibrary.MakeVector` _returnvalue _returnvalue _returnvalue)))))

(fn `DetachAllSelectedObjects`
  (bind _selectedobjects (`self.SelectedObjects`))
  (while (> (`KismetArrayLibrary.Array_Length` _selectedobjects) 0)
    (`self.RemoveFromSelection` (`|GetArrayItem` _selectedobjects))))

(fn `GetGrabbedAxis`
  (params (AxisHit :type "PrimitiveComponent Object Reference"))
  (returns (AxisGrabbed :type "EAxis Enum"))
  (if (== AxisHit (`self.XAxis`))
    (return "X")
    (elif (== AxisHit (`self.YAxis`))
      (return "Y")
      (elif (== AxisHit (`self.ZAxis`))
        (return "Z")
        (else
          (return "None"))))))

(fn `MoveWithoutMovingSelectedObjects`
  (params (NewLocation :type "Vector Structure"))
  ;[1 0 0] Detach without deselecting
  (for _array_element (`self.SelectedObjects`)
    (`self.K2_DetachFromActor` _array_element "KeepWorld" "KeepWorld" "KeepWorld"))
  ;[0 0 1] Move
  (`self.K2_SetActorLocation` NewLocation false true)
  ;[0 1 0] Reattach all selected
  (for _array_element_2 (`self.SelectedObjects`)
    (`self.K2_AttachToActor` _array_element_2 self "None" "KeepWorld" "KeepWorld" "KeepWorld" false)))

(fn `RemoveFromSelection`
  (params (VTTObject :type "/Game/VTTObject/BP_VTTObject Object Reference"))
  (bind _selectedobjects (`self.SelectedObjects`))
  (`self.K2_DetachFromActor` VTTObject "KeepWorld" "KeepWorld" "KeepWorld")
  (`KismetArrayLibrary.Array_Remove` _selectedobjects (`KismetArrayLibrary.Array_Find` _selectedobjects VTTObject))
  (`/Game/VTTObject/BP_VTTObject.Deselect` VTTObject)
  (`self.K2_AttachToActor` VTTObject (`/Game/VTTObject/BP_VTTObject.Parent` VTTObject) "None" "KeepWorld" "KeepWorld" "KeepWorld" false))

(fn `TryToAddToSelection`
  (params (VTTObject :type "/Game/VTTObject/BP_VTTObject Object Reference"))
  (returns (Selected :type Boolean))
  (bind _selected (`/Game/VTTObject/BP_VTTObject.TryToSelect` VTTObject))
  (if _selected
    (bind _returnvalue (`self.K2_AttachToActor` VTTObject self "None" "KeepWorld" "KeepWorld" "KeepWorld" false))
    (if _returnvalue
      (`KismetArrayLibrary.Array_Add` (`self.SelectedObjects`) VTTObject)
      (`self.MoveWithoutMovingSelectedObjects` (`self.K2_GetActorLocation` VTTObject))
      (return true))
    (else
      (return false))))

(fn `Update Transforms Of Selected Objects`
  (for _array_element (`self.SelectedObjects`)
    (`/Game/VTTObject/BP_VTTObject.UpdateTransform` _array_element)))

(fn `UserConstructionScript`)