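; BP_FogOfWar is a placeable actor that defines the bounds of the fog of war through its own transform.
; UpdateFogOfWarBounds writes the actor's location and its scale, converted by a factor of 100, into the FogPosition and FogSize vectors of MPC_PlayerPosition.
; It runs from the construction script and again on BeginPlay, with no per-frame update.
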(event `self.ReceiveBeginPlay`
  (`self.UpdateFogOfWarBounds`))

(fn `UpdateFogOfWarBounds`
  (`KismetMaterialLibrary.SetVectorParameterValue` "/Game/LineOfSight/MPC_PlayerPosition.MPC_PlayerPosition" "FogPosition" (`KismetMathLibrary.Conv_VectorToLinearColor` (`self.K2_GetActorLocation`)))
  (`KismetMaterialLibrary.SetVectorParameterValue` "/Game/LineOfSight/MPC_PlayerPosition.MPC_PlayerPosition" "FogSize" (`KismetMathLibrary.Conv_VectorToLinearColor` (* (`self.GetActorScale3D`) 100))))

(fn `UserConstructionScript`
  (`self.UpdateFogOfWarBounds`))