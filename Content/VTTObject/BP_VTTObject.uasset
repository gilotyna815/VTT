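; BP_VTTObject is a tabletop object with a size-based space, reach and selection state.
; The construction script looks up Size in SizeToSpaceAndReach to size and raise the space sphere, doubling the value for the reach sphere.
; It then destroys whichever collider the TakesSpace or HasReach flag disables.
; TryToSelect succeeds only for selectable, unselected objects, while Deselect and IsSelected clear and report that state.
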(fn `Deselect`
  (set `self.Selected` false))

(fn `IsSelected`
  (returns (Selected :type Boolean))
  (return (`self.Selected`)))

(fn `TryToSelect`
  (returns (Selected :type Boolean))
  (if (`self.Selected`)
    (return false) ; Already selected
    (else
      (bind _output_get (set `self.Selected` (`self.Selectable`)))
      (return _output_get))))

(fn `UserConstructionScript`
  (bind (_value _returnvalue) (`BlueprintMapLibrary.Map_Find` (`self.SizeToSpaceAndReach`) (`self.Size`)))
  (bind _returnvalue_2 (`KismetMathLibrary.SelectFloat` _value 0.0 _returnvalue))
  (bind _returnvalue_3 (* 2 _returnvalue_2))
  (`SphereComponent.SetSphereRadius` (`self.SpaceCollider`) _returnvalue_2 (`self.TakesSpace`))
  (`SceneComponent.K2_AddRelativeLocation` (`self.SpaceCollider`) (`KismetMathLibrary.MakeVector` 0.0 0.0 (/ _returnvalue_2 2.0)) false false)
  (`SphereComponent.SetSphereRadius` (`self.ReachCollider`) _returnvalue_3 (`self.HasReach`))
  (`SceneComponent.K2_AddRelativeLocation` (`self.ReachCollider`) (`KismetMathLibrary.MakeVector` 0.0 0.0 (/ _returnvalue_3 2.0)) false false)
  (if (not (`self.TakesSpace`))
    (`ActorComponent.K2_DestroyComponent` (`self.SpaceCollider`)))
  (if (not (`self.HasReach`))
    (`ActorComponent.K2_DestroyComponent` (`self.ReachCollider`))))